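; BP_ElevatorButton is a trigger button that signals elevator actors when something enters or leaves its Box.
; Each overlap event gathers all actors implementing ElevationBPI and filters them by the class held in ElevatorNumber.
; It sends ElevationMessage to each match through the interface, true on begin overlap and false on end overlap, with no check on the overlapping actor.
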(event OnComponentBeginOverlap(Box)
  (params (OverlappedComponent :type Primitive%20Component%20Object%20Reference) (OtherActor :type Actor%20Object%20Reference) (OtherComp :type Primitive%20Component%20Object%20Reference) (OtherBodyIndex :type Integer) (bFromSweep :type Boolean) (SweepResult :type Hit%20Result%20Structure%20%28by%20ref%29))
  (bind _outactors (Actor|GetAllActorswithInterface "/Game/Own/Blueprints/ElevationBPI.ElevationBPI_C"))
  (bind _filteredarray (Utilities|Array|FilterArray _outactors (Variables|Default|GetElevatorNumber)))
  (for _array_element _filteredarray
    (Class|ElevationBPI|Elevation(Message) _array_element true)))

(event OnComponentEndOverlap(Box)
  (params (OverlappedComponent :type Primitive%20Component%20Object%20Reference) (OtherActor :type Actor%20Object%20Reference) (OtherComp :type Primitive%20Component%20Object%20Reference) (OtherBodyIndex :type Integer))
  (bind _outactors (Actor|GetAllActorswithInterface "/Game/Own/Blueprints/ElevationBPI.ElevationBPI_C"))
  (bind _filteredarray (Utilities|Array|FilterArray _outactors (Variables|Default|GetElevatorNumber)))
  (for _array_element _filteredarray
    (Class|ElevationBPI|Elevation(Message) _array_element false)))

(fn ConstructionScript)