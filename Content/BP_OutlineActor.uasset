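; BP_OutlineActor toggles a red outline mesh in response to the player character's EDP_Outline event dispatcher, bound at BeginPlay.
; When enabled, it spawns a collision-free static mesh of Mesh at the parent actor's root transform, with a dynamic M_Outline_Inst material whose thickness comes from Scale.
; When disabled, it destroys that component, with HasOutline guarding against duplicates.
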(event Custom|EDP_Outline_Event_1
  (params (Outline :type Boolean))
  (if Outline
    ;[0 0 0] Create new mesh with material
    (if (not (Variables|Default|GetHasOutline))
      (bind _returnvalue (AddComponent|AddStaticMeshComponent true (Transformation|GetWorldTransform (Variables|/Script/Engine.Actor|GetRootComponent (Actor|GetParentActor)))))
      (Collision|SetCollisionEnabled _returnvalue "NoCollision")
      (bind _output_get (Variables|Default|SetNewMeshComponent _returnvalue))
      (Components|StaticMesh|SetStaticMesh _returnvalue (Variables|Default|GetMesh))
      (bind _returnvalue_2 (Rendering|Material|CreateDynamicMaterialInstance _output_get 0 "/Game/M_Outline_Inst.M_Outline_Inst" "None" :!class /Script/Engine.PrimitiveComponent))
      (Rendering|Material|SetScalarParameterValue _returnvalue_2 "Thickness" (Variables|Default|GetScale) :!class /Script/Engine.MaterialInstanceDynamic)
      (Rendering|Material|SetVectorParameterValue _returnvalue_2 "Color" "(R=0.859375,G=0.000000,B=0.000000,A=1.000000)" :!class /Script/Engine.MaterialInstanceDynamic)
      (Variables|Default|SetHasOutline true))
    (else
      ;[0 0 0] Remove component
      (Utilities|IsValid (Variables|Default|GetNewMeshComponent)
        (:Is%20Valid
          (Components|DestroyComponent (Variables|Default|GetNewMeshComponent))
          (Variables|Default|SetHasOutline false))))))

(event EventBeginPlay
  (bind _asthird_person_character (Utilities|Casting|CastToThirdPersonCharacter (Game|GetPlayerCharacter 0)))
  (EventDispatchers|AssignEDPOutline _asthird_person_character (delegate Custom|EDP_Outline_Event_1)))

(event Collision|EventActorBeginOverlap
  (params (OtherActor :type Actor%20Object%20Reference)))

(fn ConstructionScript)