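; Dummy is a Blueprint for a cube object that can display a translucent clone and an outline of itself.
; On BeginPlay it copies the Cube mesh to the Clone and Outline components and applies their translucent and outline materials.
; The Moving event toggles Clone visibility, and a separate handler toggles Outline.
; That handler's binding to the player character's EDPShowOutline dispatcher is unreachable, with an unresolved cast.
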(event Custom|EDP_ShowOutline_Event_0
  (params (Outline :type Boolean))
  ;[0 0 0 0.556] Show Outline
  (if Outline
    (Rendering|SetVisibility (Variables|Default|GetOutline) true false)
    (else
      (Rendering|SetVisibility (Variables|Default|GetOutline) false false))))

(event EventBeginPlay
  (bind _cube (Variables|Character|GetCube))
  (bind _clone (Variables|Default|GetClone))
  (bind _outline (Variables|Default|GetOutline))
  (bind _staticmesh (Variables|/Script/Engine.StaticMeshComponent|GetStaticMesh _cube))
  ;[1 1 1] Set clone mesh
  (Components|StaticMesh|SetStaticMesh _clone _staticmesh)
  (Components|StaticMesh|SetStaticMesh _outline _staticmesh)
  (Rendering|Material|SetMaterial _clone 0 "/Game/Materials/MI_Translucent.MI_Translucent")
  (Rendering|Material|SetMaterial _outline 0 "/Game/Materials/MI_Outline_Inst.MI_Outline_Inst"))

(event EventMoving
  (params (Moving :type Boolean))
  (bind _clone (Variables|Default|GetClone))
  ;[1 1 1] Show Clone
  (if Moving
    (Rendering|SetVisibility _clone true false)
    (else
      (Rendering|SetVisibility _clone false false))))

(fn ConstructionScript)