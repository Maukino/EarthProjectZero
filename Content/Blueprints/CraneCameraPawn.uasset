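; Possessable crane camera pawn for picking up and repositioning objects with the mouse, limited by a move count.
; While possessed, Tick traces under the cursor and drags the selected actor, grid-snapped inside a bounding box and raised above the hit point.
; Dropping at a new XY spends a move; running out or pressing Q repossesses the Player, and ButtonPressed adds moves.
; Timelines swing the camera between side views; click-held axes rotate it freely.
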(event EventButtonPressed
  (params (ButtonPresses :type Integer))
  ;[0 0 0 0.446] Changed 02/29 by Alex. Implemented limited crane moves functionality.
  (bind _result (Math|Integer|IncrementInt (Variables|Default|GetRemainingMoves))))

(event EventUnpossessed
  (params (OldController :type Controller%20Object%20Reference))
  ;[0 0 0 0.556] Toggle viewpoint
  (Variables|Default|SetImInCharge false)
  (Variables|/Script/Engine.PlayerController|SetbShowMouseCursor (Game|GetPlayerController 0) false))

(event EventPossessed
  (params (NewController :type Controller%20Object%20Reference))
  ;[0 0 0 0.556] Toggle viewpoint
  (Variables|Default|SetImInCharge true)
  (Variables|/Script/Engine.PlayerController|SetbShowMouseCursor (Game|GetPlayerController 0) true))

(event EventTick
  (params (DeltaSeconds :type Float%20%28single-precision%29))
  (bind _returnvalue (Game|GetPlayerController 0))
  (bind _returnvalue_2 (Game|GetPlayerController 0))
  (bind _selectedactor (Variables|Default|GetSelectedActor))
  (bind _boundingboxorigin (Variables|Default|GetBoundingBoxOrigin))
  (bind _boundingboxextent (Variables|Default|GetBoundingBoxExtent))
  (bind _grid_size (Variables|Default|GetGrid%20Size))
  (bind (_worldlocation _worlddirection) (Game|Player|ConvertMouseLocationToWorldSpace _returnvalue))
  (bind (_worldlocation_2 _worlddirection_2) (Game|Player|ConvertMouseLocationToWorldSpace _returnvalue_2))
  (bind _returnvalue_3 (* _worlddirection_2 8e+04))
  (bind _returnvalue_4 (+ _returnvalue_3 _worlddirection_2))
  ;[0 0 0 0.556 26] Event Tick
  ;[0 0 0 0.556] Linetrace to check for object to pickup
  (if (Variables|Default|GetImInCharge)
    (if (not (< (Variables|Default|GetRemainingMoves) 1))
      (Rendering|Debug|DrawDebugLine _worldlocation_2 _returnvalue_4 "(R=1.000000,G=0.042413,B=0.000000,A=1.000000)" 0.0 0.2)
      (bind _outhit (Collision|LineTraceByChannel _worldlocation_2 _returnvalue_4 "TraceTypeQuery2" false 0 "None"))
      (bind _output_get (Variables|Default|SetHoveredActor (.HitActor (Collision|BreakHitResult _outhit))))
      (bind _outhit_2 (Collision|LineTraceByChannel _worldlocation (+ (* _worlddirection 8e+04) _worlddirection) "TraceTypeQuery2" false (Utilities|Array|MakeArray (Variables|Default|GetSelectedActor)) "None"))
      (Rendering|Debug|DrawDebugBox _boundingboxorigin _boundingboxextent "(R=0.035673,G=1.000000,B=0.000000,A=1.000000)" "0, 0, 0" 0.0 5.0)
      (if (Math|Geometry|IsPointinBox (.Location (Collision|BreakHitResult _outhit_2)) _boundingboxorigin _boundingboxextent)
        (Utilities|IsValid _selectedactor
          (:Is%20Valid
            (Transformation|SetActorLocation _selectedactor (Math|Vector|MakeVector (Math|Float|SnapToGrid(Float) (.X (Math|Vector|BreakVector (.Location (Collision|BreakHitResult _outhit_2)))) _grid_size) (Math|Float|SnapToGrid(Float) (.Y (Math|Vector|BreakVector (.Location (Collision|BreakHitResult _outhit_2)))) _grid_size) (+ (.Z (Math|Vector|BreakVector (.Location (Collision|BreakHitResult _outhit_2)))) 5e+02)) true false)))))))

(event Input|ActionEvents|InputActionClick
  (params (Key :type Key%20Structure :default "None"))
  ;[0 0 0 0.556] Rotate Axis
  (:Pressed
    (Variables|Default|SetClickHeld true))
  (:Released
    (Variables|Default|SetClickHeld false)))

(event Input|ActionEvents|InputActionShowOutline
  (params (Key :type Key%20Structure :default "None"))
  (bind _player (Variables|Default|GetPlayer))
  ;[0 0 0 0.556] Show object that can be picked up
  (:Pressed
    (Default|CallEDPShowOutline _player true))
  (:Released
    (Default|CallEDPShowOutline _player false)))

(event Input|ActionEvents|InputActionRotateCameraLeft
  (params (Key :type Key%20Structure :default "None"))
  ;[0 0 0 0.556] Camera Roration
  (:Pressed
    (if (Variables|Default|GetMovedRight)
      (Development|PrintString "uwu left")
      (bind _newtrack_0 (Timeline|Timeline_1 Reverse)
        (:Update
          (Transformation|SetActorLocation _newtrack_0 false false)
          (Transformation|SetActorRotation "-40.000000, 0, 0"))
        (:Finished
          (Variables|Default|SetMovedRight false)
          (Variables|Default|SetMovedLeft false)))
      (else
        (Development|PrintString "uwu left left")
        (bind _newtrack_0_2 (Timeline|Timeline_2 Play)
          (:Update
            (Transformation|SetActorLocation _newtrack_0_2 false false)
            (Transformation|SetActorRelativeRotation "-40.000000,90.000000, 0"))
          (:Finished
            (Variables|Default|SetMovedLeft true)
            (Variables|Default|SetMovedRight false)))))))

(event Input|ActionEvents|InputActionRotateCameraRight
  (params (Key :type Key%20Structure :default "None"))
  ;[0 0 0 0.556] Camera Roration
  (:Pressed
    (if (Variables|Default|GetMovedLeft)
      (Development|PrintString "uwu left left")
      (bind _newtrack_0 (Timeline|Timeline_3 Reverse)
        (:Update
          (Transformation|SetActorLocation _newtrack_0 false false)
          (Transformation|SetActorRelativeRotation "-40.000000,0.000000, 0"))
        (:Finished
          (Variables|Default|SetMovedRight false)
          (Variables|Default|SetMovedLeft false)))
      (else
        (Development|PrintString "uwu")
        (bind _newtrack_0_2 (Timeline|Timeline_0 Play)
          (:Update
            (Transformation|SetActorLocation _newtrack_0_2 false false)
            (Transformation|SetActorRelativeRotation "-40.000000,-90.000000, 0"))
          (:Finished
            (Variables|Default|SetMovedRight true)
            (Variables|Default|SetMovedLeft false)))))))

(event Input|AxisEvents|InputAxisRotateHori
  (params (AxisValue :type Float%20%28single-precision%29))
  ;[0 0 0 0.556] Rotate Axis
  (if (Variables|Default|GetClickHeld)
    (Class|Actor|AddActorWorldRotation (Math|Rotator|MakeRotator 0.0 0.0 (* AxisValue (Variables|Default|GetCameraRotattionSpeed))))))

(event Input|AxisEvents|InputAxisRotateVert
  (params (AxisValue :type Float%20%28single-precision%29))
  ;[0 0 0 0.556] Rotate Axis
  (if (Variables|Default|GetClickHeld)
    (Transformation|AddActorLocalRotation (Math|Rotator|MakeRotator 0.0 (* AxisValue (Variables|Default|GetCameraRotattionSpeed)) 0.0) false false)))

(event Input|MouseEvents|LeftMouseButton
  (params (Key :type Key%20Structure :default "None"))
  ;[0 0 0 0.556 26] Left Mouse Button
  (:Pressed
    ;[0 0 0 0.446] Changed 02/29 by Alex. Implemented limited crane moves functionality.
    ;;[0 0 0 0.446] Pickup object
    (bind _output_get (Variables|Default|SetSelectedActor (Variables|Default|GetHoveredActor)))
    (Variables|Default|SetSelected%20Actor%20Startingpoint (Transformation|GetActorLocation _output_get))
    (Utilities|IsValid (Variables|Default|GetSelectedActor)
      (:Is%20Valid
        (Class|BPIMovable|Moving(Message) (Variables|Default|GetSelectedActor) true)
        (Rendering|SetVisibility (Variables|/Script/Engine.StaticMeshActor|GetStaticMeshComponent (Variables|Default|GetBP_Grid)) true true))))
  (:Released
    ;;[0 0 0 0.446] Drop object
    (Class|BPIMovable|Moving(Message) (Variables|Default|GetSelectedActor) false)
    (if (== (.x (Variables|Default|GetSelected%20Actor%20Startingpoint)) (.x (Transformation|GetActorLocation (Variables|Default|GetSelectedActor))))
      (if (== (.y (Variables|Default|GetSelected%20Actor%20Startingpoint)) (.y (Transformation|GetActorLocation (Variables|Default|GetSelectedActor))))
        (Variables|Default|SetSelectedActor 0)
        (Rendering|SetVisibility (Variables|/Script/Engine.StaticMeshActor|GetStaticMeshComponent (Variables|Default|GetBP_Grid)) true true)
        (else
          (Rendering|SetVisibility (Variables|/Script/Engine.StaticMeshActor|GetStaticMeshComponent (Variables|Default|GetBP_Grid)) false true :!label _label)
          (Variables|Default|SetSelectedActor 0)
          (bind _result (Math|Integer|DecrementInt (Variables|Default|GetRemainingMoves))
            (:%20%20
              (if (< _result 1)
                (Pawn|Possess (Game|GetPlayerController 0) (Variables|Default|GetPlayer)))))))
      (else
        (goto _label)))))

(event Input|KeyboardEvents|Q
  (params (Key :type Key%20Structure :default "None"))
  ;[0 0 0 0.556] Toggle viewpoint
  ;;[0 0 0 0.556] Input Q
  (:Pressed
    (Pawn|Possess (Game|GetPlayerController 0) (Variables|Default|GetPlayer))))

(event Input|MouseEvents|MouseWheelUp
  (params (Key :type Key%20Structure :default "None"))
  ;[0 0 0 0.556 26] Mouse Wheel Up/Down - Move object in zAxis
  (:Pressed
    (Variables|Default|SetSelectedActorZ (+ (Variables|Default|GetSelectedActorZ) 1e+02))))

(event Input|MouseEvents|MouseWheelDown
  (params (Key :type Key%20Structure :default "None"))
  ;[0 0 0 0.556 26] Mouse Wheel Up/Down - Move object in zAxis
  (:Pressed
    (Variables|Default|SetSelectedActorZ (+ (Variables|Default|GetSelectedActorZ) -1e+02))))

(fn ConstructionScript)

(fn CameraClamps)